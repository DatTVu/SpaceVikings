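; Player controller that creates the WBP_HUD widget on BeginPlay, adds it to the viewport and keeps a reference to it.
; Its OnManaChanged event forwards the current mana to the HUD's stamina progress update against a fixed maximum, and OnExhaustion triggers the HUD's exhaustion update.
; Both relays act only while the HUD is valid.
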(event EventBeginPlay
  (bind _returnvalue (UserInterface|CreateWidget "/Game/UI/WBP_HUD.WBP_HUD_C" self))
  (Utilities|IsValid _returnvalue
    (:Is%20Valid
      (bind _output_get (Variables|Default|SetUserHUD _returnvalue))
      (UserInterface|Viewport|AddtoViewport _output_get 0))))

(event EventTick
  (params (DeltaSeconds :type Float%20%28single-precision%29)))

(event EventOnManaChanged
  (params (currentMana :type Float%20%28single-precision%29))
  (bind _userhud (Variables|Default|GetUserHUD)
    (:then
      (Default|UpdateStaminiProgress _userhud currentMana 1e+02))
    (:else)))

(event EventOnExhaustion
  (bind _userhud (Variables|Default|GetUserHUD)
    (:then
      (Default|UpdateExhaustion _userhud))
    (:else)))

(fn ConstructionScript)