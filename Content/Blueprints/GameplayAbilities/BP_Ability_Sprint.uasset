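; Gameplay ability that makes a CharacterBase sprint while its input is held.
; On activation it raises the walk speed, applies BP_Effect_Sprint to the owner and stores the effect handle.
; A WaitInputRelease task resets the speed and ends the ability on release.
; OnEndAbility also restores the hard-coded walk speed and removes the sprint effect.
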(event Ability|EventActivateAbility
  (bind _ascharacter_base (Utilities|Casting|CastToCharacterBase (.owneractor (Ability|GetActorInfo)))
    (:then
      (Variables|Default|SetAs%20Character%20Base%20Ref _ascharacter_base)
      (Ability|Tasks|WaitInputRelease true
        (:then
          (Development|PrintString "Sprint Pressed")
          (bind _charactermovement (Variables|/Script/Engine.Character|GetCharacterMovement (Variables|Default|GetAs%20Character%20Base%20Ref))
            (:then
              (Variables|/Script/Engine.CharacterMovementComponent|SetMaxWalkSpeed _charactermovement 1e+03)
              (bind _abilitysystemcomponent (Variables|/Script/SpaceVikings.CharacterBase|GetAbilitySystemComponent (Variables|Default|GetAs%20Character%20Base%20Ref))
                (:then
                  (bind _returnvalue (GameplayEffects|ApplyGameplayEffectSpecToTarget _abilitysystemcomponent (GameplayEffects|MakeOutgoingSpec _abilitysystemcomponent "/Game/Blueprints/GameplayAbilities/BP_Effect_Sprint.BP_Effect_Sprint_C" 1.0 (GameplayEffects|MakeEffectContext _abilitysystemcomponent)) _abilitysystemcomponent))
                  (Variables|Default|SetSprintEffectHandle _returnvalue))
                (:else)))
            (:else)))
        (:OnRelease
          (Development|PrintString "Sprint Released")
          (bind _charactermovement_2 (Variables|/Script/Engine.Character|GetCharacterMovement (Variables|Default|GetAs%20Character%20Base%20Ref))
            (:then
              (Variables|/Script/Engine.CharacterMovementComponent|SetMaxWalkSpeed _charactermovement_2 6e+02)
              (Ability|EndAbility))
            (:else)))))
    (:CastFailed
      (Ability|EndAbility))))

(event Ability|EventOnEndAbility
  (params (bWasCancelled :type Boolean))
  (bind _charactermovement (Variables|/Script/Engine.Character|GetCharacterMovement (Variables|Default|GetAs%20Character%20Base%20Ref))
    (:then
      (Variables|/Script/Engine.CharacterMovementComponent|SetMaxWalkSpeed _charactermovement 6e+02)
      (bind _abilitysystemcomponent (Variables|/Script/SpaceVikings.CharacterBase|GetAbilitySystemComponent (Variables|Default|GetAs%20Character%20Base%20Ref))
        (:then
          (GameplayEffects|RemoveActiveGameplayEffect _abilitysystemcomponent (Variables|Default|GetSprintEffectHandle) -1))
        (:else)))
    (:else)))